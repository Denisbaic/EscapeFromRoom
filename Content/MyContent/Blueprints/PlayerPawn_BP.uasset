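; Player pawn that lets the player pick up world objects, browse them in an inventory widget and drop them again.
; A contact sphere tracks the overlapped PickUpObject_Base, which handles its own pickup when Use is pressed.
; CallInventory toggles the widget and mouse cursor.
; DropInventory resets the selected slot's button and array entry, restoring the object's visibility, collision and physics in front of the pawn.
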(event OnComponentBeginOverlap(PickUp_Contact_Sphere)
  (params (OverlappedComponent :type Primitive%20Component%20Object%20Reference) (OtherActor :type Actor%20Object%20Reference) (OtherComp :type Primitive%20Component%20Object%20Reference) (OtherBodyIndex :type Integer) (bFromSweep :type Boolean) (SweepResult :type Hit%20Result%20Structure%20%28by%20ref%29))
  (bind _aspick_up_object_base (Utilities|Casting|CastToPickUpObject_Base OtherActor))
  (Variables|Default|SetbCanPickUpObject true)
  (bind _output_get (Variables|Default|SetObjectToPickUp _aspick_up_object_base))
  (Variables|/Game/MyContent/Blueprints/PickUpObject_Base.PickUpObject_Base_C|SetPlayer_That_Picked_Object_Up _output_get self))

(event OnComponentEndOverlap(PickUp_Contact_Sphere)
  (params (OverlappedComponent :type Primitive%20Component%20Object%20Reference) (OtherActor :type Actor%20Object%20Reference) (OtherComp :type Primitive%20Component%20Object%20Reference) (OtherBodyIndex :type Integer))
  (Utilities|Casting|CastToPickUpObject_Base OtherActor)
  (Variables|Default|SetbCanPickUpObject false)
  (Variables|Default|SetObjectToPickUp 0))

(event EventBeginPlay
  (bind _returnvalue (UserInterface|CreateWidget "/Game/MyContent/Widgets/Inventory_W.Inventory_W_C"))
  (bind _output_get (Variables|Default|SetInventoryVar _returnvalue))
  (Default|SetArrayButton _output_get))

(event Collision|EventActorBeginOverlap
  (params (OtherActor :type Actor%20Object%20Reference)))

(event EventTick
  (params (DeltaSeconds :type Float%20%28single-precision%29)))

(event Input|ActionEvents|InputActionUse
  (params (Key :type Key%20Structure))
  (:Pressed
    (if (Variables|Default|GetbCanPickUpObject)
      (Default|ObjectPickedUp (Variables|Default|GetObjectToPickUp)))))

(event Input|ActionEvents|InputActionCallInventory
  (params (Key :type Key%20Structure))
  (bind _returnvalue (Game|GetPlayerController 0))
  (:Pressed
    (Utilities|FlowControl|FlipFlop
      (:A
        (Variables|/Script/Engine.PlayerController|SetbShowMouseCursor _returnvalue true)
        (UserInterface|Viewport|AddtoViewport (Variables|Default|GetInventoryVar) 0))
      (:B
        (Variables|/Script/Engine.PlayerController|SetbShowMouseCursor _returnvalue false)
        (Widget|RemovefromParent (Variables|Default|GetInventoryVar))))))

(event Input|ActionEvents|InputActionDropInventory
  (params (Key :type Key%20Structure))
  (bind _inventoryvar (Variables|Default|GetInventoryVar))
  (bind _inventoryarray (Variables|Default|GetInventoryArray))
  (bind _inventoryvar_2 (Variables|Default|GetInventoryVar))
  (bind _selectedslot (Variables|/Game/MyContent/Widgets/Inventory_W.Inventory_W_C|GetSelectedSlot _inventoryvar_2))
  (bind _selectedslot_2 (Variables|/Game/MyContent/Widgets/Inventory_W.Inventory_W_C|GetSelectedSlot _inventoryvar))
  (:Pressed
    (if (!= (Utilities|Array|Get(acopy) (Variables|Default|GetInventoryArray) _selectedslot) 0)
      (Class|Button|SetStyle (Utilities|Array|Get(acopy) (Variables|/Game/MyContent/Widgets/Inventory_W.Inventory_W_C|GetButtonsArray _inventoryvar_2) _selectedslot) (Utilities|Struct|MakeButtonStyle "(ImageSize=(X=32.000000,Y=32.000000),Margin=(Left=0.000000,Top=0.000000,Right=0.000000,Bottom=0.000000),Tint=(R=1.000000,G=1.000000,B=1.000000,A=1.000000),TintColor=(SpecifiedColor=(R=1.000000,G=1.000000,B=1.000000,A=1.000000),ColorUseRule=UseColor_Specified),ResourceObject=None,ResourceName=\"\",UVRegion=(Min=(X=0.000000,Y=0.000000),Max=(X=0.000000,Y=0.000000),bIsValid=0),DrawAs=Image,Tiling=NoTile,Mirroring=NoMirror,ImageType=NoImage,bIsDynamicallyLoaded=False,bHasUObject=False)" "(ImageSize=(X=32.000000,Y=32.000000),Margin=(Left=0.000000,Top=0.000000,Right=0.000000,Bottom=0.000000),Tint=(R=1.000000,G=1.000000,B=1.000000,A=1.000000),TintColor=(SpecifiedColor=(R=1.000000,G=1.000000,B=1.000000,A=1.000000),ColorUseRule=UseColor_Specified),ResourceObject=None,ResourceName=\"\",UVRegion=(Min=(X=0.000000,Y=0.000000),Max=(X=0.000000,Y=0.000000),bIsValid=0),DrawAs=Image,Tiling=NoTile,Mirroring=NoMirror,ImageType=NoImage,bIsDynamicallyLoaded=False,bHasUObject=False)"))
      (Utilities|ShowObject (Utilities|Array|Get(acopy) _inventoryarray _selectedslot_2))
      (Utilities|Array|SetArrayElem _inventoryarray _selectedslot_2 0))))

(fn ConstructionScript)