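; Door Blueprint that swings open and closed and shows its state through a spotlight color.
; On BeginPlay it binds custom events to the open and close delegates of its OpenDoor member, which supplies the trigger.
; Opening turns the light green and plays a timeline that drives the door's relative yaw.
; Closing turns the light red and reverses the same timeline.
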(event Custom|DoorOpenEvent_Event_0
  (Rendering|Components|Light|SetLightColor (Variables|Default|GetSpotLight) "(R=0.000000,G=1.000000,B=0.024492,A=1.000000)" true)
  (bind _door_angle (Timeline|Timeline_0 Play)
    (:Update
      (Transformation|SetRelativeRotation (Variables|Default|GetDoor) (Math|Rotator|MakeRotator 0.0 0.0 _door_angle) false false))))

(event Custom|DoorCloseEvent_Event_0
  (Rendering|Components|Light|SetLightColor (Variables|Default|GetSpotLight) "(R=1.000000,G=0.000000,B=0.000000,A=1.000000)" true)
  (bind _door_angle (Timeline|Timeline_0 Reverse)
    (:Update
      (Transformation|SetRelativeRotation (Variables|Default|GetDoor) (Math|Rotator|MakeRotator 0.0 0.0 _door_angle) false false))))

(event EventBeginPlay
  (EventDispatchers|AssignDoorOpenEvent (Variables|Default|GetOpenDoor) (delegate Custom|DoorOpenEvent_Event_0))
  (EventDispatchers|AssignDoorCloseEvent (Variables|Default|GetOpenDoor) (delegate Custom|DoorCloseEvent_Event_0)))

(event Collision|EventActorBeginOverlap
  (params (OtherActor :type Actor%20Object%20Reference)))

(event EventTick
  (params (DeltaSeconds :type Float%20%28single-precision%29)))

(fn ConstructionScript)