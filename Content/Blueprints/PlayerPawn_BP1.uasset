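; PlayerPawn_BP1 is a player pawn that grabs physics objects in front of it with the GetItem input.
; A press line-traces PhysicsBody objects forward from the collision component up to InteractionDistance, along a ray that Tick draws as a debug arrow.
; A hit teleports HeldObjectSlot to the impact point, joins it to the component by physics constraint and makes that component ignore Pawn collision.
; DropObject, called while holding, is an empty stub.
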(event EventBeginPlay)

(event Collision|EventActorBeginOverlap
  (params (OtherActor :type Actor%20Object%20Reference)))

(event EventTick
  (params (DeltaSeconds :type Float%20%28single-precision%29))
  (bind _collisioncomponent (Variables|Default|GetCollisionComponent))
  (bind _returnvalue (Transformation|GetWorldLocation _collisioncomponent))
  (Rendering|Debug|DrawDebugArrow :LineStart _returnvalue :LineEnd (+ _returnvalue (* (Math|Vector|GetForwardVector _collisioncomponent) (Variables|Default|GetInteractionDistance))) :ArrowSize 1e+02 :Duration 1.0))

(event Input|ActionEvents|InputActionGetItem
  (params (Key :type Key%20Structure))
  (:Pressed
    (Utilities|IsValid (Variables|Default|GetHeldObject)
      (:Is%20Valid
        (CallFunction|DropObject))
      (:Is%20Not%20Valid
        (bind (_hitresult _ishitsomething) (CallFunction|TraceObjects))
        (if _ishitsomething
          (CallFunction|GrabObject _hitresult))))))

(fn ConstructionScript)

(fn TraceObjects
  (bind _collisioncomponent (Variables|Default|GetCollisionComponent))
  (bind _returnvalue (Transformation|GetWorldLocation _collisioncomponent))
  (bind (_outhit _returnvalue_2) (Collision|LineTraceForObjects _returnvalue (+ _returnvalue (* (Math|Vector|GetForwardVector _collisioncomponent) (Variables|Default|GetInteractionDistance))) (Utilities|Array|MakeArray "ObjectTypeQuery4") false 0 "None"))
  (return _outhit _returnvalue_2))

(fn GrabObject
  (params (HitResult :type Hit%20Result%20Structure))
  (bind (_bblockinghit _binitialoverlap _time _distance _location _impactpoint _normal _impactnormal _physmat _hitactor _hitcomponent _hitbonename) (Collision|BreakHitResult HitResult))
  (Transformation|SetWorldLocation (Variables|Default|GetHeldObjectSlot) _impactpoint false true)
  (Class|PhysicsConstraintComponent|SetConstrainedComponents (Variables|Default|GetPhysicsConstraint) (Variables|Default|GetHeldObjectSlot) "None" _hitcomponent _hitbonename)
  (Collision|SetCollisionResponsetoChannel _hitcomponent "ECC_Pawn" "ECR_Ignore")
  (Variables|Default|SetHeldObject _hitcomponent))

(fn DropObject)