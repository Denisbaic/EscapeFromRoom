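; Base Blueprint for objects that can be picked up into a player's inventory.
; ObjectPickedUp puts the object in the first matching (apparently empty) slot of the player's InventoryArray and restyles the inventory button at that index.
; HideObject then hides the static mesh and disables its physics and collision, so the actor is stored rather than destroyed.
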(event Custom|ObjectPickedUp
  (bind _basebuttonstyle (Variables|Default|GetBaseButtonStyle))
  (bind (_array_element _array_index) (Utilities|Array|ForEachLoopwithBreak (Variables|/Game/Blueprints/PlayerPawn_BP.PlayerPawn_BP_C|GetInventoryArray (Variables|Default|GetPlayer_That_Picked_Object_Up)) :!label _label)
    (:LoopBody
      (if (== _array_element 0)
        (Utilities|Array|SetArrayElem (Variables|/Game/Blueprints/PlayerPawn_BP.PlayerPawn_BP_C|GetInventoryArray (Variables|Default|GetPlayer_That_Picked_Object_Up)) _array_index self)
        (Class|Button|SetStyle (Utilities|Array|Get(acopy) (Variables|/Game/Widgets/Inventory_W.Inventory_W_C|GetButtonsArray (Variables|/Game/Blueprints/PlayerPawn_BP.PlayerPawn_BP_C|GetInventoryVar (Variables|Default|GetPlayer_That_Picked_Object_Up))) _array_index) (Utilities|Struct|MakeButtonStyle _basebuttonstyle _basebuttonstyle _basebuttonstyle))
        (Utilities|HideObject)
        (goto _label Break)))))

(fn ConstructionScript)