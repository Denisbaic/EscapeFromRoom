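; Door actor that opens and closes on events from its CheckPlayerInvDoor component, which by its name checks the player's inventory.
; BeginPlay binds both events, then runs the close handler so the door starts in its closed state.
; Opening turns the spotlight green and plays a timeline that drives the door's yaw.
; Closing turns the light red and reverses that same timeline.
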(event Custom|DoorOpenEvent_0
  (Rendering|Components|Light|SetLightColor (Variables|Default|GetSpotLight) "(R=0.000000,G=1.000000,B=0.024492,A=1.000000)" true)
  (bind _door_angle (Timeline|Timeline_1 Play)
    (:Update
      (Transformation|SetRelativeRotation (Variables|Default|GetDoor) (Math|Rotator|MakeRotator 0.0 0.0 _door_angle) false false))))

(event Custom|DoorCloseEvent_0
  (Rendering|Components|Light|SetLightColor (Variables|Default|GetSpotLight) "(R=1.000000,G=0.000000,B=0.000000,A=1.000000)" true)
  (bind _door_angle (Timeline|Timeline_1 Reverse)
    (:Update
      (Transformation|SetRelativeRotation (Variables|Default|GetDoor) (Math|Rotator|MakeRotator 0.0 0.0 _door_angle) false false))))

(event EventBeginPlay
  (|CallParentFunction)
  (EventDispatchers|AssignDoorOpenEvent (Variables|Default|GetCheckPlayerInvDoor) (delegate Custom|DoorOpenEvent_0))
  (EventDispatchers|AssignDoorCloseEvent (Variables|Default|GetCheckPlayerInvDoor) (delegate Custom|DoorCloseEvent_0))
  (CallFunction|DoorCloseEvent0))

(event Collision|EventActorBeginOverlap
  (params (OtherActor :type Actor%20Object%20Reference))
  (|CallParentFunction OtherActor) ; This node is disabled and will not be called.\nDrag off pins to build functionality.
)

(event EventTick
  (params (DeltaSeconds :type Float%20%28single-precision%29))
  (|CallParentFunction DeltaSeconds) ; This node is disabled and will not be called.\nDrag off pins to build functionality.
)

(fn ConstructionScript
  (|CallParentFunction))